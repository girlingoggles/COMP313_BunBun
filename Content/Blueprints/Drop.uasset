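; Drop is a wandering pickup that changes BunBun's color, restores a little health and destroys itself on overlap.
; Any overlap credits the player pawn without checking the overlapping actor, and plays an explosion sound at the direction vector.
; It decrements BunBun's DropCount, spawning a replacement at a random reachable point around the player when one or fewer remain.
; Tick feeds movement with a random horizontal vector, rerolled on a looping delay.
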(event Custom|onSpawn
  (bind _returnvalue (Math|Random|RandomUnitVector))
  (bind (_x _y) (Math|Vector|BreakVector _returnvalue))
  (bind _output_get (Variables|Default|Setdrop_vector (Math|Vector|MakeVector _x _y 0.0) :!label _label))
  (Utilities|FlowControl|Delay 5.0)
  (goto _label))

(event EventBeginPlay
  (bind _returnvalue (Math|Random|RandomUnitVector))
  (bind (_x _y) (Math|Vector|BreakVector _returnvalue))
  (bind _output_get (Variables|Default|Setdrop_vector (Math|Vector|MakeVector _x _y 0.0) :!label _label))
  (Utilities|FlowControl|Delay 5.0)
  (goto _label))

(event EventTick
  (params (DeltaSeconds :type Float%20%28single-precision%29))
  (Class|PawnMovementComponent|AddInputVector (Variables|Default|GetDrop_move) (stale Custom|onSpawn _output_get) false))

(event Collision|EventActorBeginOverlap
  (params (OtherActor :type Actor%20Object%20Reference))
  (bind _asbun_bun (Utilities|Casting|CastToBunBun (Game|Player|GetPlayerPawn 0)))
  (AddComponent|AddBunBunColor _asbun_bun)
  (Audio|PlaySoundatLocation "/Game/StarterContent/Audio/Explosion02.Explosion02" (Variables|Default|Getdrop_vector) "0, 0, 0" 1.0 1.0 0.0 0 0 0)
  (Utilities|FlowControl|Delay 0.1)
  (AddComponent|AddBunBunColor _asbun_bun)
  (Actor|DestroyActor)
  (Variables|/Game/Blueprints/BunBun.BunBun_C|SetHealth _asbun_bun (+ (Variables|/Game/Blueprints/BunBun.BunBun_C|GetHealth _asbun_bun) 0.1))
  (bind _output_get (Variables|/Game/Blueprints/BunBun.BunBun_C|Setdrop_count _asbun_bun (- (Variables|/Game/Blueprints/BunBun.BunBun_C|Getdrop_count _asbun_bun) 1)))
  (Math|Integer|CompareInt _output_get 1
    (:==
      _)
    (:<
      _))
  (bind _returnvalue (Game|SpawnActorfromClass "Drop_C" (Math|Transform|MakeTransform (.RandomLocation (AI|Navigation|GetRandomReachablePointinRadius (Transformation|GetActorLocation _asbun_bun) 2e+03 0 0)) "0, 0, 0" "0.500000,0.500000,0.500000") "Undefined" 0 0))
  (Variables|/Game/Blueprints/BunBun.BunBun_C|Setdrop_count _asbun_bun (+ (Variables|/Game/Blueprints/BunBun.BunBun_C|Getdrop_count _asbun_bun) 1))
  (CallFunction|OnSpawn _returnvalue))

(event Collision|EventHit
  (params (MyComp :type Primitive%20Component%20Object%20Reference) (Other :type Actor%20Object%20Reference) (OtherComp :type Primitive%20Component%20Object%20Reference) (bSelfMoved :type Boolean) (HitLocation :type Vector :default "0, 0, 0") (HitNormal :type Vector :default "0, 0, 0") (NormalImpulse :type Vector :default "0, 0, 0") (Hit :type Hit%20Result%20Structure%20%28by%20ref%29)))

(fn ConstructionScript)