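; BunBun is a physics-driven player character moved by axis-input impulses on BunBunMesh for horizontal movement and jumping.
; Tick caps horizontal velocity while preserving vertical speed, then drains Health whenever horizontal movement input is nonzero.
; After each drain, it adds a WIN widget if Health is at least one or a DIE widget if at most zero, with no guard against repeats.
; Overlap and hit events are empty.
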(event OnComponentHit(BunBunMesh)
  (params (HitComponent :type Primitive%20Component%20Object%20Reference) (OtherActor :type Actor%20Object%20Reference) (OtherComp :type Primitive%20Component%20Object%20Reference) (NormalImpulse :type Vector :default "0, 0, 0") (Hit :type Hit%20Result%20Structure%20%28by%20ref%29)))

(event Collision|EventActorBeginOverlap
  (params (OtherActor :type Actor%20Object%20Reference)))

(event EventTick
  (params (DeltaSeconds :type Float%20%28single-precision%29))
  (bind _returnvalue (Transformation|GetVelocity))
  (bind (_x _y _z) (Math|Vector|BreakVector _returnvalue))
  (bind _returnvalue_2 (Math|Vector|MakeVector _x _y 0.0))
  (bind _returnvalue_3 (Math|Vector|ClampVectorSize _returnvalue_2 0.0 2e+03))
  (bind (_x_2 _y_2) (Math|Vector|BreakVector _returnvalue_3))
  (Physics|SetPhysicsLinearVelocity (Variables|Default|GetBunBunMesh) (Math|Vector|MakeVector _x_2 _y_2 _z) false "None")
  (Math|Float|CompareFloat (.X (Math|Vector|BreakVector (* (+ (Math|Vector|MakeVector 0.0 (stale Input|AxisEvents|InputAxisMoveLR AxisValue) 0.0) (Math|Vector|MakeVector (stale Input|AxisEvents|InputAxisMoveFB AxisValue) 0.0 0.0)) (Variables|Default|GetStrength)))) 0.0
    (:>
      _)
    (:==
      (Math|Float|CompareFloat (.Y (Math|Vector|BreakVector (* (+ (Math|Vector|MakeVector 0.0 (stale Input|AxisEvents|InputAxisMoveLR AxisValue) 0.0) (Math|Vector|MakeVector (stale Input|AxisEvents|InputAxisMoveFB AxisValue) 0.0 0.0)) (Variables|Default|GetStrength)))) 0.0
        (:>
          _)
        (:==
          (Math|Float|CompareFloat (.Z (Math|Vector|BreakVector (* (+ (Math|Vector|MakeVector 0.0 (stale Input|AxisEvents|InputAxisMoveLR AxisValue) 0.0) (Math|Vector|MakeVector (stale Input|AxisEvents|InputAxisMoveFB AxisValue) 0.0 0.0)) (Variables|Default|GetStrength)))) 0.0
            (:>
              _)
            (:<
              _)))
        (:<
          _)))
    (:<
      _))
  (bind _output_get (Variables|Default|SetHealth (- (Variables|Default|GetHealth) 0.0005)))
  (Math|Float|CompareFloat _output_get 0.0
    (:>
      (Math|Float|CompareFloat _output_get 1.0
        (:>
          _)
        (:==
          _))
      (bind _returnvalue_4 (UserInterface|CreateWidget "/Game/Blueprints/WIN.WIN_C"))
      (UserInterface|Viewport|AddtoViewport _returnvalue_4 0))
    (:==
      (bind _returnvalue_5 (UserInterface|CreateWidget "/Game/Blueprints/DIE.DIE_C" :!label _label))
      (UserInterface|Viewport|AddtoViewport _returnvalue_5 0))
    (:<
      (goto _label))))

(event Input|AxisEvents|InputAxisMoveFB
  (params (AxisValue :type Float%20%28single-precision%29))
  (Physics|AddImpulse (Variables|Default|GetBunBunMesh) (* (+ (Math|Vector|MakeVector 0.0 (stale Input|AxisEvents|InputAxisMoveLR AxisValue) 0.0) (Math|Vector|MakeVector AxisValue 0.0 0.0)) (Variables|Default|GetStrength)) "None" false))

(event Input|AxisEvents|InputAxisMoveLR
  (params (AxisValue :type Float%20%28single-precision%29))
  (Physics|AddImpulse (Variables|Default|GetBunBunMesh) (* (+ (Math|Vector|MakeVector 0.0 AxisValue 0.0) (Math|Vector|MakeVector (stale Input|AxisEvents|InputAxisMoveFB AxisValue) 0.0 0.0)) (Variables|Default|GetStrength)) "None" false))

(event Input|AxisEvents|InputAxisMoveJump
  (params (AxisValue :type Float%20%28single-precision%29))
  (Physics|AddImpulse (Variables|Default|GetBunBunMesh) (Math|Vector|MakeVector 0.0 0.0 (* (Variables|Components|GetMaxSpeed) AxisValue)) "None" false))

(event Input|KeyboardEvents|Gravity
  (params (AxisValue :type Vector :default "0, 0, 0"))
  (Physics|AddImpulse (Variables|Default|GetBunBunMesh) (Math|Vector|MakeVector 0.0 0.0 (* (Variables|Components|GetMaxSpeed) (stale Input|AxisEvents|InputAxisMoveJump AxisValue))) "None" false))

(fn ConstructionScript)